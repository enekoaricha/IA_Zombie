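; BP_ZombieCharacter is an AI zombie character that detects pawns and exposes attack and movement speed controls.
; When its PawnSensing component sees a pawn, it sets IsDetected and stores that pawn as PlayerTarget in the blackboard.
; The Attack event forwards its value to the anim_zombie animation instance.
; UpdateSpeed changes the movement component's max walk speed only when the value differs.
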(event `Attack`
  (params (Attack :type Boolean))
  (bind _asanim_zombie (cast `/Game/Animation/anim_zombie` (`SkeletalMeshComponent.GetAnimInstance` (`self.Mesh`))))
  (set `/Game/Animation/anim_zombie.attack` Attack _asanim_zombie))

(event `self.PawnSensing.OnSeePawn`
  (params (Pawn :type "Pawn Object Reference"))
  (bind _returnvalue (`AIBlueprintHelperLibrary.GetBlackboard` null))
  (`BlackboardComponent.SetValueAsBool` _returnvalue "IsDetected" true)
  (`BlackboardComponent.SetValueAsObject` _returnvalue "PlayerTarget" Pawn))

(fn `UpdateSpeed`
  (params (Speed :type "Float (double-precision)"))
  (bind _charactermovement (`self.CharacterMovement`))
  (if (== Speed (`CharacterMovementComponent.MaxWalkSpeed` _charactermovement))
    (return)
    (else
      (set `CharacterMovementComponent.MaxWalkSpeed` Speed _charactermovement)
      (return))))

(fn `UserConstructionScript`)